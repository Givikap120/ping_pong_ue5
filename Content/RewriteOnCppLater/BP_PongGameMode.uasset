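; Pong game mode Blueprint that tracks goals and drives the score display.
; On BeginPlay it creates the UI_Score widget and binds every GoalTrigger's OnGoalScored event to its goal handler.
; For player IDs 0 or 1, the handler increments the widget's score for that side and resets the Ball found in the level.
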(event `self.ReceiveBeginPlay`
  (bind _returnvalue (`|CreateWidget` "/Game/UI/UI_Score.UI_Score_C"))
  (`UserWidget.AddToViewport` _returnvalue 0)
  (set `self.ScoreWidget` _returnvalue)
  (bind _outactors (`GameplayStatics.GetAllActorsOfClass` "/Script/Ping_Pong.GoalTrigger"))
  (for _array_element _outactors
    (add `GoalTrigger.OnGoalScored` _array_element (delegate `HandleGoalScore`))))

(event `HandleGoalScore`
  (params (PlayerID :type Integer))
  (bind _returnvalue (== PlayerID 1))
  (if (or (== PlayerID 0) _returnvalue)
    (`/Game/UI/UI_Score.IncrementScore` (`self.ScoreWidget`) _returnvalue)
    (bind _returnvalue_2 (`GameplayStatics.GetActorOfClass` "/Script/Ping_Pong.Ball"))
    (`Ball.ResetBall` _returnvalue_2)))

(fn `UserConstructionScript`)