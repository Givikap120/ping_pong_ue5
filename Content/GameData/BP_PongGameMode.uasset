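; BP_PongGameMode is the game mode for a two-player Pong game, handling match start and score updates.
; On login it registers the player, and once two controllers exist it calls StartGame on each, then resets the ball after a short delay.
; When a goal is scored it runs the parent handler, then pushes both players' scores to every BP_PongController.
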(event `self.HandleGoalScored`
  (params (PlayerId :type Integer))
  (`parent.HandleGoalScored` PlayerId)
  (bind _outactors (`GameplayStatics.GetAllActorsOfClass` "/Game/GameData/BP_PongController.BP_PongController_C"))
  (for _array_element _outactors
    (`/Game/GameData/BP_PongController.UpdateScore` _array_element (`self.Player0_Score`) (`self.Player1_Score`))))

(event `self.K2_PostLogin`
  (params (NewPlayer :type "PlayerController Object Reference"))
  (`self.HandleNewPlayer` NewPlayer)
  (if (== (`KismetArrayLibrary.Array_Length` (`self.Controllers`)) 2)
    (for _array_element (`self.Controllers`)
      (bind _asbp_pong_controller (cast `/Game/GameData/BP_PongController` _array_element))
      (`/Game/GameData/BP_PongController.StartGame` _asbp_pong_controller))
    (`KismetSystemLibrary.Delay` 0.2)
    (`Ball.ResetBall` (`self.Ball`))))

(fn `UserConstructionScript`)