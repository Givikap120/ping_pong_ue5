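; BP_PongController is the player controller for a Pong game, managing each player's waiting and score UI.
; On BeginPlay, a local controller shows a wait-for-player widget unless the game has already started.
; StartGame flags the game as started, swaps that widget for a score widget, and UpdateScore forwards both players' scores to it.
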(event `UpdateScore`
  (params (`Player0 Score` :type Integer) (`Player1 Score` :type Integer))
  (`/Game/UI/UI_Score.UpdateScore` (`self.Score Widget`) `Player0 Score` `Player1 Score`))

(event `StartGame`
  (bind _wait_widget (`self.Wait Widget`))
  (set `self.IsGameStarted` true)
  (`/Engine/EditorBlueprintResources/StandardMacros.IsValid` _wait_widget
    (:`Is Valid`
      (`Widget.RemoveFromParent` _wait_widget))
    (:`Is Not Valid`
      _))
  (bind _returnvalue (`|CreateWidget` "/Game/UI/UI_Score.UI_Score_C"))
  (`UserWidget.AddToViewport` _returnvalue 0)
  (set `self.Score Widget` _returnvalue))

(event `self.ReceiveBeginPlay`
  (if (and (`self.IsLocalController`) (not (`self.IsGameStarted`)))
    (bind _returnvalue (`|CreateWidget` "/Game/UI/UI_WaitForPlayer.UI_WaitForPlayer_C"))
    (`UserWidget.AddToViewport` _returnvalue 0)
    (set `self.Wait Widget` _returnvalue)))

(fn `UserConstructionScript`)